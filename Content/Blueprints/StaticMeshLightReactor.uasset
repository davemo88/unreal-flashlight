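; An actor that reacts to BotPawn overlaps by stretching along its Y axis.
; Begin and end overlap events from a BotPawn set an Overlapped flag.
; Tick grows the Y scale in fixed steps up to a cap while overlapped, then shrinks it back toward normal size otherwise, independent of frame time.
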(event EventBeginPlay)

(event Collision|EventActorBeginOverlap
  (params (OtherActor :type Actor%20Object%20Reference))
  (Utilities|Casting|CastToBotPawn OtherActor)
  (Variables|Default|SetbOverlapped true))

(event EventTick
  (params (DeltaSeconds :type Float%20%28single-precision%29))
  (bind _returnvalue (Transformation|GetActorScale3D))
  (bind (_x _y _z) (Math|Vector|BreakVector _returnvalue))
  (if (Variables|Default|GetbOverlapped)
    (if (< _y 5.0)
      (Transformation|SetActorScale3D (Math|Vector|MakeVector _x (+ _y 0.1) _z)))
    (elif (> _y 1.0)
      (Transformation|SetActorScale3D (Math|Vector|MakeVector _x (- _y 0.1) _z)))))

(event Collision|EventActorEndOverlap
  (params (OtherActor :type Actor%20Object%20Reference))
  (Utilities|Casting|CastToBotPawn OtherActor)
  (Variables|Default|SetbOverlapped false))

(fn ConstructionScript)