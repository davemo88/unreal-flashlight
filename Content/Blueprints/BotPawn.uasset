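; BotPawn is an input-driven pawn that moves forward and back, turns, and tilts its head.
; MoveForward adds movement input along the control rotation's yaw, while Turn feeds controller yaw.
; LookUp adds the axis value to the Head component's relative pitch without clamping, zeroing roll and yaw.
; LookRight is empty, and leftover nodes for head yaw, world-axis movement and facing velocity are disconnected.
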(event EventBeginPlay)

(event EventTick
  (params (DeltaSeconds :type Float%20%28single-precision%29)))

(event Input|AxisEvents|InputAxisMoveForward
  (params (AxisValue :type Float%20%28single-precision%29))
  (Pawn|Input|AddMovementInput (Math|Vector|GetForwardVector (Math|Rotator|MakeRotator 0.0 0.0 (.Yaw (Math|Rotator|BreakRotator (Pawn|GetControlRotation :!class /Script/Engine.Pawn))))) AxisValue false))

(event Input|AxisEvents|InputAxisLookUp
  (params (AxisValue :type Float%20%28single-precision%29))
  (bind _head (Variables|Default|GetHead))
  (Transformation|SetRelativeRotation _head (Math|Rotator|MakeRotator 0.0 (+ (.Pitch (Math|Rotator|BreakRotator (.Rotation (Math|Transform|BreakTransform (Transformation|GetRelativeTransform _head))))) AxisValue) 0.0) false false))

(event Input|AxisEvents|InputAxisTurn
  (params (AxisValue :type Float%20%28single-precision%29))
  (Pawn|Input|AddControllerYawInput AxisValue))

(event Input|AxisEvents|InputAxisLookRight
  (params (AxisValue :type Float%20%28single-precision%29)))

(fn ConstructionScript)